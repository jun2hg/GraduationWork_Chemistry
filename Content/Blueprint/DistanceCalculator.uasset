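; Gaze-accuracy logger that scores how close the VR pawn's view lands to the origin of the actor it hits.
; A looping one-second timer line-traces forward from the VR camera and maps impact-to-actor-origin distance to a clamped score, highest at the center.
; Scores are printed and appended to a string, which is saved to a text file on EndPlay.
; An unconnected branch holds a first-person camera alternative.
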(event `self.ReceiveBeginPlay`
  ;[1 1 1] VR_Pawn
  (bind _asvr_pawn (cast `/Game/Blueprint/VR_Pawn` (`GameplayStatics.GetPlayerPawn` 0)))
  (set `self.VR Camera` (`/Game/Blueprint/VR_Pawn.VR_Camera` _asvr_pawn))
  (`KismetSystemLibrary.K2_SetTimer` null "CalculateAndSaveDists" 1.0 true))

(event `self.ReceiveEndPlay`
  (params (EndPlayReason :type "EEndPlayReason Enum" :default "Destroyed"))
  ;[1 1 1] Save File
  (`BPFL_SaveFile.SaveTextToFile` (`self.N_Dists_String`) "test.txt"))

(fn `CalculateAndSaveDists`
  (bind _vr_camera (`self.VR Camera`))
  (bind _returnvalue (`SceneComponent.K2_GetComponentLocation` _vr_camera))
  (bind _outhit (`KismetSystemLibrary.LineTraceSingle` :`Start` _returnvalue :`End` (+ _returnvalue (* (`KismetMathLibrary.GetForwardVector` (`SceneComponent.K2_GetComponentRotation` _vr_camera)) 1500.0)) :`TraceChannel` "TraceTypeQuery1" :`DrawDebugType` "ForOneFrame"))
  (bind (_bblockinghit _binitialoverlap _time _distance _location _impactpoint _normal _impactnormal _physmat _hitactor) (`GameplayStatics.BreakHitResult` _outhit))
  (bind _output_get (set `self.Normalized_Dist` (`KismetMathLibrary.Lerp` 1000.0 0.0 (`KismetMathLibrary.FClamp` (/ (`KismetMathLibrary.Vector_Distance` _impactpoint (`self.K2_GetActorLocation` _hitactor)) 400.0)))))
  (bind _output_get_2 (set `self.N_Dists_String` (`KismetStringLibrary.Concat_StrStr` (`self.N_Dists_String`) (`KismetStringLibrary.Concat_StrStr` (`KismetStringLibrary.Conv_DoubleToString` _output_get) " \n"))))
  (`KismetSystemLibrary.PrintString` _output_get_2))

(fn `UserConstructionScript`)