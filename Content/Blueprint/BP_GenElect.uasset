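; BP_GenElect is a spawner that fills a box volume with electron actors.
; Two custom events, Generate_Electrons and Generate_Electrons10, each loop a fixed number of times to spawn BP_Electron or BP_Electron10 respectively, then call Spawned on each new actor.
; Spawn locations are random points within the Box component's scaled extent, centered on its center of mass.
; BeginPlay is empty, and nothing in this Blueprint calls either event.
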(event `Generate_Electrons`
  (bind _box (`self.Box`))
  (for _ (range 16)
    (bind _returnvalue (`|SpawnActorFromClass` "/Game/Blueprint/BP_Electron.BP_Electron_C" (`KismetMathLibrary.MakeTransform` (`KismetMathLibrary.RandomPointInBoundingBox` (`PrimitiveComponent.GetCenterOfMass` _box "None") (`BoxComponent.GetScaledBoxExtent` _box))) "Undefined" "MultiplyWithRoot" null null))
    (`/Game/Blueprint/BP_Electron.Spawned` _returnvalue)))

(event `self.ReceiveBeginPlay`)

(event `Generate_Electrons10`
  (bind _box (`self.Box`))
  (for _ (range 11)
    (bind _returnvalue (`|SpawnActorFromClass` "/Game/Blueprint/BP_Electron10.BP_Electron10_C" (`KismetMathLibrary.MakeTransform` (`KismetMathLibrary.RandomPointInBoundingBox` (`PrimitiveComponent.GetCenterOfMass` _box "None") (`BoxComponent.GetScaledBoxExtent` _box))) "Undefined" "MultiplyWithRoot" null null))
    (`/Game/Blueprint/BP_Electron10.Spawned` _returnvalue)))

(fn `UserConstructionScript`)